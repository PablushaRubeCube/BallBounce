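; BP_Brick is a breakable brick for the BallBounce game that takes hits until its lives run out.
; On BeginPlay it binds a hit-count widget to itself and picks blue material for single-life bricks, yellow otherwise.
; BrickHit decrements lives with a sound; the final hit decrements the game mode's block count, adds score to the game instance and destroys the brick.
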(event EventBrickHit
  (CallFunction|DicrementLives))

(event EventBeginPlay
  (bind _returnvalue (UserInterface|CreateWidget "/Game/BallBounce/HUD/W_NumberOfHitBrick.W_NumberOfHitBrick_C"))
  (Variables|/Game/BallBounce/HUD/W_NumberOfHitBrick.W_NumberOfHitBrick_C|SetRefToBrick _returnvalue self)
  (UserInterface|SetWidget (Variables|Default|GetNumber) _returnvalue)
  (if (== (Variables|Default|GetlivesBrick) 1)
    (Rendering|Material|SetMaterial (Variables|Default|GetBrickMesh) 0 "/Game/StarterContent/Materials/M_Basic_Wall_Blue.M_Basic_Wall_Blue")
    (else
      (Rendering|Material|SetMaterial (Variables|Default|GetBrickMesh) 0 "/Game/StarterContent/Materials/M_Basic_Yellow.M_Basic_Yellow"))))

(fn ConstructionScript)

(fn DicrementLives
  (if (< (- (Variables|Default|GetlivesBrick) 1) 1)
    (Audio|PlaySound2D "/Game/Retro_8Bit_Sounds/Collectables/Cues/retro_collect_pickup_coin_10_Cue.retro_collect_pickup_coin_10_Cue" 1.0 1.0 0.0 0 0)
    (bind _asball_bounce_game_mode (Utilities|Casting|CastToBallBounceGameMode (Game|GetGameMode)))
    (Default|DicrementBlock _asball_bounce_game_mode)
    (bind _asbp_ball_game_instance (Utilities|Casting|CastToBP_BallGameInstance (Game|GetGameInstance)))
    (Math|Integer|IncrementInt (Variables|/Game/BallBounce/Blueprints/BP_BallGameInstance.BP_BallGameInstance_C|GetScore _asbp_ball_game_instance)
      (:%20%20
        (Actor|DestroyActor)))
    (else
      (Audio|PlaySound2D "/Game/Retro_8Bit_Sounds/Collectables/Cues/retro_collect_pickup_coin_09_Cue.retro_collect_pickup_coin_09_Cue" 1.0 1.0 0.0 0 0)
      (Math|Integer|DecrementInt (Variables|Default|GetlivesBrick)))))