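; Ball actor for a brick-breaker style game, bouncing off paddles, bricks and other surfaces.
; A game mode start-playing event resets it to a fixed spot with a randomized direction.
; In one game state, Tick moves it by swept offsets, unscaled by delta time, reflecting off hit normals.
; Paddle hits play a sound and skew the bounce by paddle input and MinX; other hits notify BPI_BrickHit implementers.
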(event Custom|StartPlayingEvent
  (CallFunction|ResetLocationOftheBall))

(event EventBeginPlay
  (bind _asball_bounce_game_mode (Utilities|Casting|CastToBallBounceGameMode (Game|GetGameMode)))
  (EventDispatchers|AssignStartPlaying _asball_bounce_game_mode (delegate Custom|StartPlayingEvent)))

(event EventTick
  (params (DeltaSeconds :type Float%20%28single-precision%29))
  ;[1 1 1] Cheak StateOfGame
  (bind _asball_bounce_game_mode (Utilities|Casting|CastToBallBounceGameMode (Game|GetGameMode)))
  (if (Utilities|Enum|Equal(Enum) (Variables|/Game/BallBounce/Blueprints/BallBounceGameMode.BallBounceGameMode_C|GetStateOfTheGame _asball_bounce_game_mode) "NewEnumerator5")
    ;[1 1 1] MoveBall
    (bind _sweephitresult (Transformation|AddActorWorldOffset (Math|Vector|MakeVector (.x (* (Variables|Default|GetDirection) (Variables|Default|GetSpeed))) (.y (* (Variables|Default|GetDirection) (Variables|Default|GetSpeed))) 0.0) true))
    (Variables|Default|SetHit%20Actor (.HitActor (Collision|BreakHitResult _sweephitresult)))
    ;[1 1 1] if Ball touch paddle
    (bind _aspaddle (Utilities|Casting|CastToPaddle (Variables|Default|GetHit%20Actor))
      (:then
        (Audio|PlaySound2D "/Game/Retro_8Bit_Sounds/Jumping/Cues/retro_jump_bounce_12_Cue.retro_jump_bounce_12_Cue" 1.0 1.0 0.0 0 0)
        (Variables|Default|SetDirection (Math|Vector|Normalize (Math|Vector|MakeVector (+ (Variables|Default|GetMinX) (.X (Math|Vector|BreakVector (Math|Vector|Normalize (Math|Vector|MakeVector (.X (Math|Vector|BreakVector (Math|Vector|GetReflectionVector (Variables|Default|GetDirection) (.ImpactNormal (Collision|BreakHitResult _sweephitresult))))) (+ (* (Variables|/Game/BallBounce/Blueprints/Paddle.Paddle_C|GetAxis%20Value _aspaddle) 5.0) (.Y (Math|Vector|BreakVector (Math|Vector|GetReflectionVector (Variables|Default|GetDirection) (.ImpactNormal (Collision|BreakHitResult _sweephitresult)))))) (.Z (Math|Vector|BreakVector (Math|Vector|GetReflectionVector (Variables|Default|GetDirection) (.ImpactNormal (Collision|BreakHitResult _sweephitresult)))))))))) (.Y (Math|Vector|BreakVector (Math|Vector|Normalize (Math|Vector|MakeVector (.X (Math|Vector|BreakVector (Math|Vector|GetReflectionVector (Variables|Default|GetDirection) (.ImpactNormal (Collision|BreakHitResult _sweephitresult))))) (+ (* (Variables|/Game/BallBounce/Blueprints/Paddle.Paddle_C|GetAxis%20Value _aspaddle) 5.0) (.Y (Math|Vector|BreakVector (Math|Vector|GetReflectionVector (Variables|Default|GetDirection) (.ImpactNormal (Collision|BreakHitResult _sweephitresult)))))) (.Z (Math|Vector|BreakVector (Math|Vector|GetReflectionVector (Variables|Default|GetDirection) (.ImpactNormal (Collision|BreakHitResult _sweephitresult))))))))) (.Z (Math|Vector|BreakVector (Math|Vector|Normalize (Math|Vector|MakeVector (.X (Math|Vector|BreakVector (Math|Vector|GetReflectionVector (Variables|Default|GetDirection) (.ImpactNormal (Collision|BreakHitResult _sweephitresult))))) (+ (* (Variables|/Game/BallBounce/Blueprints/Paddle.Paddle_C|GetAxis%20Value _aspaddle) 5.0) (.Y (Math|Vector|BreakVector (Math|Vector|GetReflectionVector (Variables|Default|GetDirection) (.ImpactNormal (Collision|BreakHitResult _sweephitresult)))))) (.Z (Math|Vector|BreakVector (Math|Vector|GetReflectionVector (Variables|Default|GetDirection) (.ImpactNormal (Collision|BreakHitResult _sweephitresult)))))))))))))
      (:CastFailed
        ;;[1 1 1] Reflection Ball
        (Variables|Default|SetDirection (Math|Vector|GetReflectionVector (Variables|Default|GetDirection) (.ImpactNormal (Collision|BreakHitResult _sweephitresult))))
        (if (Utilities|DoesObjectImplementInterface (Variables|Default|GetHit%20Actor) "/Game/BallBounce/Blueprints/BPI_BrickHit.BPI_BrickHit_C")
          (Class|BPIBrickHit|BrickHit(Message) (Variables|Default|GetHit%20Actor)))))))

(fn ConstructionScript)

(fn ResetLocationOftheBall
  (Transformation|SetActorLocation "640.000000,0.000000, 0" false false)
  (Variables|Default|SetDirection (Math|Vector|Normalize (Math|Vector|MakeVector 1.0 (Math|Random|RandomFloatinRange -1.0 1.0) 0.0))))