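; Game mode for a brick-breaker game that drives match flow through a state machine, from ready and countdown through play to game over or completion.
; Tick runs the three-second countdown, then entering Playing calls StartPlaying.
; It counts BP_Brick actors at BeginPlay; clearing them opens the next numbered level or completes the game.
; Oops checks game-instance lives to retry or end; both endings show the quit widget.
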(event Custom|SetStateOfTheGame
  (params (StateOfTheGame :type StateOfGame%20Enum :default "NewEnumerator0"))
  ;[1 1 1] ChoseState
  (switch Utilities|FlowControl|Switch|SwitchonStateOfGame StateOfTheGame
    (:NewEnumerator0
      (Variables|Default|SetStateOfTheGame StateOfTheGame :!label _label))
    (:NewEnumerator1
      (Variables|Default|SetCountDown 3.0)
      (goto _label))
    (:NewEnumerator2
      ;;[1 1 1] Oops!
      (Variables|Default|SetStateOfTheGame "NewEnumerator2")
      (Utilities|FlowControl|Delay 1.5)
      (bind _asbp_ball_game_instance (Utilities|Casting|CastToBP_BallGameInstance (Game|GetGameInstance)))
      (if (< (Variables|/Game/BallBounce/Blueprints/BP_BallGameInstance.BP_BallGameInstance_C|GetLive _asbp_ball_game_instance) 1)
        (CallFunction|SetStateOftheGame "NewEnumerator3")
        (Utilities|FlowControl|Delay 0.5)
        (CallFunction|Ooops!NewGame)
        (else
          (CallFunction|SetStateOftheGame "NewEnumerator0"))))
    (:NewEnumerator3
      (goto _label))
    (:NewEnumerator4
      ;;[1 1 1] LevelComplited!
      (Variables|Default|SetStateOfTheGame "NewEnumerator4")
      (Utilities|FlowControl|Delay 0.5)
      (bind _asbp_ball_game_instance_2 (Utilities|Casting|CastToBP_BallGameInstance (Game|GetGameInstance)))
      (if (== (Variables|/Game/BallBounce/Blueprints/BP_BallGameInstance.BP_BallGameInstance_C|GetCurrentLevel _asbp_ball_game_instance_2) (Variables|/Game/BallBounce/Blueprints/BP_BallGameInstance.BP_BallGameInstance_C|GetMaxLevel _asbp_ball_game_instance_2))
        (CallFunction|SetStateOftheGame "NewEnumerator6")
        (else
          (bind _result (Math|Integer|IncrementInt (Variables|/Game/BallBounce/Blueprints/BP_BallGameInstance.BP_BallGameInstance_C|GetCurrentLevel _asbp_ball_game_instance_2))
            (:%20%20
              (Game|OpenLevel(byName) (Utilities|String|StringToName (Utilities|String|Append "Level" (Utilities|String|ToString(Integer) _result)))))))))
    (:NewEnumerator5
      (Variables|Default|SetStateOfTheGame "NewEnumerator5")
      (Default|CallStartPlaying))
    (:NewEnumerator6
      (Variables|Default|SetStateOfTheGame "NewEnumerator6")
      (Utilities|FlowControl|Delay 1.5)
      (CallFunction|Ooops!NewGame))))

(event EventBeginPlay
  ;[1 1 1] StartState
  (CallFunction|SetStateOftheGame "NewEnumerator0")
  (bind _outactors (Actor|GetAllActorsOfClass "/Game/BallBounce/Blueprints/BP_Brick.BP_Brick_C"))
  (for _array_element _outactors
    (Math|Integer|IncrementInt (Variables|Default|GetBlockCount))))

(event EventTick
  (params (DeltaSeconds :type Float%20%28single-precision%29))
  ;[1 1 1] BeginCountDownState
  (if (Utilities|Enum|Equal(Enum) (Variables|Default|GetStateOfTheGame) "NewEnumerator1")
    (Variables|Default|SetCountDown (- (Variables|Default|GetCountDown) DeltaSeconds))
    (if (> (- (Variables|Default|GetCountDown) DeltaSeconds) 2.0)
      (Variables|Default|SetCount 3)
      (elif (> (Variables|Default|GetCountDown) 1.0)
        (Variables|Default|SetCount 2)
        (elif (> (Variables|Default|GetCountDown) 0.0)
          (Variables|Default|SetCount 1)
          (else
            (CallFunction|SetStateOftheGame "NewEnumerator5")))))))

(fn ConstructionScript)

(fn Ooops!NewGame
  (bind _returnvalue (Game|GetPlayerController 0))
  (bind _returnvalue_2 (UserInterface|CreateWidget "/Game/BallBounce/HUD/WBP_QuitGame.WBP_QuitGame_C"))
  (UserInterface|Viewport|AddtoViewport _returnvalue_2 0)
  (Variables|/Script/Engine.PlayerController|SetbShowMouseCursor _returnvalue true)
  (Input|SetInputModeUIOnly _returnvalue _returnvalue_2 "DoNotLock"))

(fn DicrementBlock
  (Math|Integer|DecrementInt (Variables|Default|GetBlockCount)
    (:%20%20
      (if (<= (Variables|Default|GetBlockCount) 0)
        (CallFunction|SetStateOftheGame "NewEnumerator4")))))