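; BallBounceController is the input controller for the BallBounce game, forwarding player actions to BallBounceGameMode.
; LMBDown advances the game mode's StateOfTheGame from its first enum value to its second, and does nothing in other states.
; Menu calls OoopsNewGame on the game mode and then pauses the game.
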(event EventBeginPlay)

(event EventTick
  (params (DeltaSeconds :type Float%20%28single-precision%29)))

(event Input|ActionEvents|InputActionLMBDown
  (params (Key :type Key%20Structure :default "None"))
  (:Pressed
    (bind _asball_bounce_game_mode (Utilities|Casting|CastToBallBounceGameMode (Game|GetGameMode)))
    (if (Utilities|Enum|Equal(Enum) (Variables|/Game/BallBounce/Blueprints/BallBounceGameMode.BallBounceGameMode_C|GetStateOfTheGame _asball_bounce_game_mode) "NewEnumerator0")
      (Default|SetStateOftheGame _asball_bounce_game_mode "NewEnumerator1"))))

(event Input|ActionEvents|InputActionMenu
  (params (Key :type Key%20Structure :default "None"))
  (:Pressed
    (bind _asball_bounce_game_mode (Utilities|Casting|CastToBallBounceGameMode (Game|GetGameMode)))
    (Default|Ooops!NewGame _asball_bounce_game_mode)
    (Game|SetGamePaused true)))

(fn ConstructionScript)