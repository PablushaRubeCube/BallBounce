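; Player paddle for the BallBounce game, moved sideways along Y by the MouseLeftRight input axis.
; Each axis event stores its value and acts only while BallBounceGameMode is in one specific game state.
; Helper functions compare the position to LeftLimit and RightLimit, allowing only inward movement past either limit, applied as a swept world offset scaled by the axis.
; An unconnected older limit check on X remains in the graph.
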(event Input|AxisEvents|InputAxisMouseLeftRight
  (params (AxisValue :type Float%20%28single-precision%29))
  (Variables|Default|SetAxis%20Value AxisValue)
  ;[1 1 1] Cheak StateOfGame
  (bind _asball_bounce_game_mode (Utilities|Casting|CastToBallBounceGameMode (Game|GetGameMode)))
  (if (Utilities|Enum|Equal(Enum) (Variables|/Game/BallBounce/Blueprints/BallBounceGameMode.BallBounceGameMode_C|GetStateOfTheGame _asball_bounce_game_mode) "NewEnumerator5")
    (if (CallFunction|IsLessThan)
      (if (CallFunction|AxisGreaterThanZero)
        (Transformation|AddActorWorldOffset (Math|Vector|MakeVector 0.0 (* (Variables|Default|GetAxis%20Value) 25.0) 0.0) true :!label _label))
      (elif (CallFunction|IsGreaterThan)
        (if (CallFunction|AxisLessThanZero)
          (goto _label))
        (else
          (goto _label))))))

(fn ConstructionScript)

(fn IsLessThan
  (return (< (.Y (Math|Vector|BreakVector (Transformation|GetActorLocation))) (Variables|Default|GetLeftLimit))))

(fn IsGreaterThan
  (return (> (.Y (Math|Vector|BreakVector (Transformation|GetActorLocation))) (Variables|Default|GetRightLimit))))

(fn AxisGreaterThanZero
  (return (> (Variables|Default|GetAxis%20Value) 0.0)))

(fn AxisLessThanZero
  (return (< (Variables|Default|GetAxis%20Value) 0.0)))